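; BP_LerpDebugColor is a debug visualization actor that shows a linear color interpolation as a row of spheres.
; On BeginPlay a loop draws ten temporary debug spheres, raising Step each pass to blend cyan to red and lift each sphere from the actor's height.
; The spheres share the actor's X, while their Y spacing is measured from world zero.
; An unconnected Timeline variant would animate a red-to-blue sphere at the actor's location.
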(event `self.ReceiveBeginPlay`
  (bind (_returnvalue_x _returnvalue_y _returnvalue_z) (`KismetMathLibrary.BreakVector` (`self.K2_GetActorLocation`)))
  (for _index (range 10)
    (`KismetSystemLibrary.DrawDebugSphere` (`KismetMathLibrary.MakeVector` _returnvalue_x (* (`KismetMathLibrary.Conv_IntToDouble` (mod _index 10)) 150.0) (+ _returnvalue_z (* (`self.step`) 1500.0))) 100.0 24 (`KismetMathLibrary.LinearColorLerp` (struct :`G` 0.816275 :`B` 1.0 :`A` 1.0) (struct :`R` 1.0 :`G` 0.037066 :`A` 1.0) (`self.step`)) 12.0 4.0)
    (set `self.step` (+ (`self.step`) 0.1))))

(fn `UserConstructionScript`)