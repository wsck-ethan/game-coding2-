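; BP_nodeInClass is a linked path node that visualizes its chain with timed debug lines.
; Its createlinks event draws differently colored lines to the valid PrevNode and NextNode actors.
; After a short delay it calls CreateLinks on NextNode, so the drawing ripples forward node by node until no valid next node remains.
; The graph comment mentions spawning a sphere at the chain's end, but no such logic exists.
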(event `create links`
  (bind _prevnode (`self.PrevNode`))
  (`/Engine/EditorBlueprintResources/StandardMacros.IsValid` _prevnode
    (:`Is Valid`
      (`KismetSystemLibrary.DrawDebugLine` (`SceneComponent.K2_GetComponentLocation` (`self.Sphere`)) (`self.K2_GetActorLocation` _prevnode) (struct :`R` 0.288266 :`G` 0.38866 :`B` 1.0 :`A` 1.0) 4.0 4.0))
    (:`Is Not Valid`
      _))
  (`/Engine/EditorBlueprintResources/StandardMacros.IsValid` (`self.NextNode`)
    (:`Is Valid`
      (`KismetSystemLibrary.DrawDebugLine` (`SceneComponent.K2_GetComponentLocation` (`self.DefaultSceneRoot`)) (`self.K2_GetActorLocation` (`self.NextNode`)) (struct :`R` 1.0 :`G` 0.457433 :`B` 0.487291 :`A` 1.0) 4.0 4.0)
      (`KismetSystemLibrary.Delay` 0.2)
      (`self.create links` (`self.NextNode`)))))

(fn `UserConstructionScript`)