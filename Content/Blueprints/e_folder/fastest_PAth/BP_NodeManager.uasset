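; BP_NodeManager grows an endless chain of BP_nodeInClass actors in the level as a doubly linked list.
; On BeginPlay it spawns the first node at its own location, then SpawnNewNode re-calls itself after a short delay.
; Each new node gets an incrementing index, a random position in a box around the last node, and Prev/Next links.
; The drawpath event, noted as spacebar-triggered, calls CreateLinks on the first node.
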(event `self.ReceiveBeginPlay`
  (bind _nodeindex (`self.NodeIndex`))
  (bind _returnvalue (`|SpawnActorFromClass` "/Game/Blueprints/e_folder/fastest_PAth/BP_nodeInClass.BP_nodeInClass_C" (`KismetMathLibrary.MakeTransform` (`self.K2_GetActorLocation`)) "Undefined" "MultiplyWithRoot" null null))
  (set `self.FirstNode` _returnvalue)
  (set `self.LastNode` _returnvalue)
  (set `/Game/Blueprints/e_folder/fastest_PAth/BP_nodeInClass.index` _nodeindex _returnvalue)
  (`/Engine/EditorBlueprintResources/StandardMacros.IncrementInt` _nodeindex
    (:`  `
      (`self.SpawnNewNode`))))

(event `SpawnNewNode`
  (bind _nodeindex (`self.NodeIndex`))
  (bind _lastnode (`self.LastNode`))
  (`KismetSystemLibrary.PrintString` "spawning a new node")
  (bind _returnvalue (`|SpawnActorFromClass` "/Game/Blueprints/e_folder/fastest_PAth/BP_nodeInClass.BP_nodeInClass_C" (`KismetMathLibrary.MakeTransform` (`KismetMathLibrary.RandomPointInBoundingBox` (`self.K2_GetActorLocation` (`self.LastNode`)) (500.0 500.0 500.0))) "Undefined" "MultiplyWithRoot" null null))
  (set `/Game/Blueprints/e_folder/fastest_PAth/BP_nodeInClass.index` _nodeindex _returnvalue)
  (`/Engine/EditorBlueprintResources/StandardMacros.IncrementInt` _nodeindex
    (:`  `
      (set `/Game/Blueprints/e_folder/fastest_PAth/BP_nodeInClass.PrevNode` _lastnode _returnvalue)
      (set `/Game/Blueprints/e_folder/fastest_PAth/BP_nodeInClass.NextNode` _returnvalue _lastnode)
      (set `self.LastNode` _returnvalue) ; setss the managets last node to be this nodes
      (`KismetSystemLibrary.Delay` 0.2)
      (`self.SpawnNewNode`))))

(event `draw path`
  (`/Game/Blueprints/e_folder/fastest_PAth/BP_nodeInClass.create links` (`self.FirstNode`)))

(fn `UserConstructionScript`)