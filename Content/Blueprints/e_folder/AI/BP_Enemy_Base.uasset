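; Base enemy Blueprint that provides a melee attack and a fire effect that can be lit and put out.
; The attack event plays a zombie right-hand attack montage and calls the OnAttackEnd dispatcher whether it completes or is interrupted.
; The spawnfire event creates a BP_Fire actor, snaps it to a hand socket on the mesh and stores it for extinguish_fire to destroy.
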(event `attack`
  (`|PlayMontage` (`self.Mesh`) "/Game/BSP_ZombieAnims/Animations/Standing/Attack/AS_NAAT_Zombie_Attack_RH_Stand_Montage.AS_NAAT_Zombie_Attack_RH_Stand_Montage"
    (:`OnCompleted`
      _)
    (:`OnInterrupted`
      _))
  (`self.OnAttackEnd`))

(event `spawn fire`
  (bind _returnvalue (`|SpawnActorFromClass` "/Game/Blueprints/BP_Fire.BP_Fire_C" (`SceneComponent.K2_GetComponentToWorld` (`self.CapsuleComponent`)) "Undefined" "MultiplyWithRoot" null null))
  (set `self.BP_fire` _returnvalue)
  (`self.K2_AttachToComponent` _returnvalue (`self.Mesh`) "hand_rFirePivot" "SnapToTarget" "SnapToTarget" "SnapToTarget" true))

(event `extinguish_fire`
  (`self.K2_DestroyActor` (`self.BP_fire`)))

(fn `UserConstructionScript`)