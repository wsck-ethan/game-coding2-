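; BP_PatrolRoute is a spline-based patrol route that supplies world-space waypoints, presumably for patrolling AI.
; Each GetPatrolPointLocation call first runs IncrementPatrolPoint, then returns the spline point at the new PatrolIndex, so reading the location advances the route.
; Direction flips at either end for back-and-forth traversal, though the upper check lets the index reach the point count, one past the last valid point.
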(event `Increment Patrol Point`
  (set `self.patrolIndex` (+ (`self.patrolIndex`) (`self.direction`)))
  ;[1 1 1] check if at end
  (if (>= (`self.patrolIndex`) (`SplineComponent.GetNumberOfSplinePoints` (`self.spline`)))
    ;[1 1 1] flip direction
    (set `self.direction` -1)
    (elif (<= (`self.patrolIndex`) 0)
      (set `self.direction` 1))))

(fn `Get patrol point location`
  (returns (location :type "Vector Structure"))
  (`self.Increment Patrol Point`)
  (return (`SplineComponent.GetLocationAtSplinePoint` (`self.spline`) (`self.patrolIndex`) "World")))

(fn `UserConstructionScript`)