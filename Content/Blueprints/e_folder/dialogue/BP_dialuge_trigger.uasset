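; BP_dialuge_trigger is a sphere trigger for an old man's dialogue, showing an E prompt widget when the player character enters.
; Delay loops poll the character's IsTalking flag, then swap the prompt for the dialogue widget and play audio, initially from the DT_dialogue row at DialogueRowIndex.
; Another polling loop resets dialogue past the last row and re-shows the prompt if still in range; leaving clears both widgets.
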(event `self.ReceiveBeginPlay`
  (bind _asbp_third_person_character (cast `/Game/ThirdPerson/Blueprints/BP_ThirdPersonCharacter` (`GameplayStatics.GetPlayerCharacter` 0)))
  (bind _returnvalue (`|CreateWidget` "/Game/Blueprints/e_folder/dialogue/Widgets/W_oldman.W_oldman_C"))
  (set `self.dialogue Widget` _returnvalue)
  (bind _returnvalue_2 (`|CreateWidget` "/Game/Blueprints/e_folder/dialogue/Widgets/W_E_dialogue.W_E_dialogue_C"))
  (set `self.E_widget` _returnvalue_2)
  (`KismetSystemLibrary.Delay` 0.2 :!label _label)
  (if (> (`/Game/ThirdPerson/Blueprints/BP_ThirdPersonCharacter.dialogue row index` _asbp_third_person_character) (`/Game/ThirdPerson/Blueprints/BP_ThirdPersonCharacter.dialogue max row index` _asbp_third_person_character))
    (set `/Game/ThirdPerson/Blueprints/BP_ThirdPersonCharacter.dialogue row index` 0 _asbp_third_person_character)
    (set `/Game/ThirdPerson/Blueprints/BP_ThirdPersonCharacter.is talking` false _asbp_third_person_character)
    (`Widget.RemoveFromParent` (`self.dialogue Widget`))
    (`self.still in sphere`)
    (goto _label)
    (else
      (goto _label))))

(event `self.Sphere.OnComponentBeginOverlap`
  (params (OverlappedComponent :type "PrimitiveComponent Object Reference") (OtherActor :type "Actor Object Reference") (OtherComp :type "PrimitiveComponent Object Reference") (OtherBodyIndex :type Integer) (bFromSweep :type Boolean) (SweepResult :type "HitResult Structure (by ref)"))
  (bind _e_widget (`self.E_widget`))
  (bind _asbp_third_person_character (cast `/Game/ThirdPerson/Blueprints/BP_ThirdPersonCharacter` OtherActor))
  (set `/Game/ThirdPerson/Blueprints/BP_ThirdPersonCharacter.is talking` false _asbp_third_person_character)
  (set `self.in sphere` true)
  (if (`/Game/ThirdPerson/Blueprints/BP_ThirdPersonCharacter.is talking` _asbp_third_person_character)
    (`Widget.RemoveFromParent` _e_widget)
    (`UserWidget.AddToViewport` (`self.dialogue Widget`) 0)
    (else
      (`UserWidget.AddToViewport` _e_widget 0)
      (`KismetSystemLibrary.Delay` 0.1 :!label _label_2)
      (if (`/Game/ThirdPerson/Blueprints/BP_ThirdPersonCharacter.is talking` _asbp_third_person_character)
        (`Widget.RemoveFromParent` _e_widget)
        (bind _outrownames (`DataTableFunctionLibrary.GetDataTableRowNames` "/Game/Blueprints/e_folder/dialogue/DT_dialogue.DT_dialogue"))
        (bind _returnvalue (`|GetDataTableRow` "/Game/Blueprints/e_folder/dialogue/DT_dialogue.DT_dialogue" (`|GetArrayItem` _outrownames (`/Game/ThirdPerson/Blueprints/BP_ThirdPersonCharacter.dialogue row index` _asbp_third_person_character)))
          (:`then`
            (`GameplayStatics.PlaySound2D` (`.audio_5_88AAA94C473C991D89EEF6B6D60BFD78` (break `/Game/Blueprints/e_folder/dialogue/S_dialogue` _returnvalue)) 1.0 1.0 0.0 null null)
            (`UserWidget.AddToViewport` (`self.dialogue Widget`) 0)))
        (elif (`self.in sphere`)
          (goto _label_2))))))

(event `self.Sphere.OnComponentEndOverlap`
  (params (OverlappedComponent :type "PrimitiveComponent Object Reference") (OtherActor :type "Actor Object Reference") (OtherComp :type "PrimitiveComponent Object Reference") (OtherBodyIndex :type Integer))
  (bind _asbp_third_person_character (cast `/Game/ThirdPerson/Blueprints/BP_ThirdPersonCharacter` (`GameplayStatics.GetPlayerCharacter` 0)))
  (set `/Game/ThirdPerson/Blueprints/BP_ThirdPersonCharacter.dialogue row index` 0 _asbp_third_person_character)
  (bind _asbp_third_person_character_2 (cast `/Game/ThirdPerson/Blueprints/BP_ThirdPersonCharacter` OtherActor))
  (`Widget.RemoveFromParent` (`self.E_widget`))
  (`Widget.RemoveFromParent` (`self.dialogue Widget`))
  (set `self.in sphere` false)
  (set `/Game/ThirdPerson/Blueprints/BP_ThirdPersonCharacter.is talking` false _asbp_third_person_character_2))

(event `check to see at end`
  (bind _asbp_third_person_character (cast `/Game/ThirdPerson/Blueprints/BP_ThirdPersonCharacter` (`GameplayStatics.GetPlayerCharacter` 0))))

(event `still in sphere`
  (bind _e_widget (`self.E_widget`))
  (if (`self.in sphere`)
    (bind _asbp_third_person_character (cast `/Game/ThirdPerson/Blueprints/BP_ThirdPersonCharacter` (`GameplayStatics.GetPlayerCharacter` 0)))
    (set `/Game/ThirdPerson/Blueprints/BP_ThirdPersonCharacter.is talking` false _asbp_third_person_character)
    (set `self.in sphere` true)
    (if (`/Game/ThirdPerson/Blueprints/BP_ThirdPersonCharacter.is talking` _asbp_third_person_character)
      (`Widget.RemoveFromParent` _e_widget)
      (`UserWidget.AddToViewport` (`self.dialogue Widget`) 0)
      (else
        (`UserWidget.AddToViewport` _e_widget 0)
        (`KismetSystemLibrary.Delay` 0.1 :!label _label_3)
        (if (`/Game/ThirdPerson/Blueprints/BP_ThirdPersonCharacter.is talking` _asbp_third_person_character)
          (`Widget.RemoveFromParent` _e_widget)
          (`UserWidget.AddToViewport` (`self.dialogue Widget`) 0)
          (`/Game/ThirdPerson/Blueprints/BP_ThirdPersonCharacter.play 2d sound` _asbp_third_person_character)
          (elif (`self.in sphere`)
            (goto _label_3)))))))

(fn `UserConstructionScript`)