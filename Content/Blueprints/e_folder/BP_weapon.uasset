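; BP_weapon is a weapon Blueprint that holds a damage range, weapon type and elemental type and displays them as text.
; The RandomizeValues event adds a random bonus to the current minimum damage, derives the maximum from it with another random offset, then calls UpdateText.
; UpdateText writes the max-min damage string and both enum names into three text elements.
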(event `randomize values`
  (bind _output_get (set `self.min damage` (+ (`self.min damage`) (`KismetMathLibrary.RandomInteger` 2))))
  (set `self.max damage` (+ _output_get (`KismetMathLibrary.RandomIntegerInRange` 1 4)))
  (`self.update text`))

(event `update text`
  (`TextRenderComponent.K2_SetText` (`self.damage`) (`KismetTextLibrary.Conv_StringToText` (`KismetStringLibrary.Concat_StrStr` (`KismetStringLibrary.Conv_IntToString` (`self.max damage`)) "max" "-" (`KismetStringLibrary.Conv_IntToString` (`self.min damage`)) "min")))
  (`TextRenderComponent.K2_SetText` (`self.weapon type`) (`KismetTextLibrary.Conv_StringToText` (`|GetEnumeratorNameAsString` (`self.weaponType`))))
  (`TextRenderComponent.K2_SetText` (`self.elemetal type`) (`KismetTextLibrary.Conv_StringToText` (`|GetEnumeratorNameAsString` (`self.elementaltype`)))))

(fn `UserConstructionScript`)