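; A trigger actor for a platform puzzle element that reacts to BP_ThirdPersonCharacter entering and leaving its Box.
; On entry it spawns a new BP_plateforms at the location of the referenced Plateform actor, with card-shuffle and chip sounds around the spawn.
; On exit it instantly moves the referenced Plateform down by a fixed offset, without sweeping; the spawned copy is not stored or removed.
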(event `self.Box.OnComponentBeginOverlap`
  (params (OverlappedComponent :type "PrimitiveComponent Object Reference") (OtherActor :type "Actor Object Reference") (OtherComp :type "PrimitiveComponent Object Reference") (OtherBodyIndex :type Integer) (bFromSweep :type Boolean) (SweepResult :type "HitResult Structure (by ref)"))
  (cast `/Game/ThirdPerson/Blueprints/BP_ThirdPersonCharacter` OtherActor)
  (`GameplayStatics.PlaySound2D` "/Game/Blueprints/e_folder/AUDIO/card-shuffle.card-shuffle" 1.0 1.0 0.0 null null)
  (`|SpawnActorFromClass` "/Game/Blueprints/e_folder/doors-puzzleitems/BP_plateforms.BP_plateforms_C" (`KismetMathLibrary.Conv_VectorToTransform` (`self.K2_GetActorLocation` (`self.plateform`))) "Undefined" "MultiplyWithRoot" null null)
  (`GameplayStatics.PlaySound2D` "/Game/Blueprints/e_folder/AUDIO/chip-lay-1.chip-lay-1" 1.0 1.0 0.0 null null))

(event `self.Box.OnComponentEndOverlap`
  (params (OverlappedComponent :type "PrimitiveComponent Object Reference") (OtherActor :type "Actor Object Reference") (OtherComp :type "PrimitiveComponent Object Reference") (OtherBodyIndex :type Integer))
  (bind _plateform (`self.plateform`))
  (cast `/Game/ThirdPerson/Blueprints/BP_ThirdPersonCharacter` OtherActor)
  (`self.K2_SetActorLocation` _plateform (+ (`self.K2_GetActorLocation` _plateform) (0.0 0.0 -400.0)) false false))

(fn `UserConstructionScript`)