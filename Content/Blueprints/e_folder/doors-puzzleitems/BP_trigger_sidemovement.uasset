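; A pressure-plate style trigger that slides a referenced Door actor sideways while the player stands in its box.
; When a BP_ThirdPersonCharacter enters the Box, it plays two 2D sounds, instantly offsets the Door along world X and adds a particle component to it.
; On exit it applies the reverse offset and plays an impact sound.
; Moves are relative, unswept snaps with no interpolation.
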(event `self.ReceiveBeginPlay`)

(event `self.Box.OnComponentBeginOverlap`
  (params (OverlappedComponent :type "PrimitiveComponent Object Reference") (OtherActor :type "Actor Object Reference") (OtherComp :type "PrimitiveComponent Object Reference") (OtherBodyIndex :type Integer) (bFromSweep :type Boolean) (SweepResult :type "HitResult Structure (by ref)"))
  (bind _door (`self.door`))
  (cast `/Game/ThirdPerson/Blueprints/BP_ThirdPersonCharacter` OtherActor)
  (`GameplayStatics.PlaySound2D` "/Game/Blueprints/e_folder/AUDIO/card-place-4.card-place-4" 1.0 1.0 0.0 null null)
  (`GameplayStatics.PlaySound2D` "/Game/Blueprints/e_folder/AUDIO/impactPlate_medium_000.impactPlate_medium_000" 1.0 1.0 0.0 null null)
  (`self.K2_SetActorLocation` _door (+ (`self.K2_GetActorLocation` _door) (400.0 0.0 0.0)) false false)
  (`AddComponent|NODE_AddParticleSystemComponent-2` :`self` _door))

(event `self.Box.OnComponentEndOverlap`
  (params (OverlappedComponent :type "PrimitiveComponent Object Reference") (OtherActor :type "Actor Object Reference") (OtherComp :type "PrimitiveComponent Object Reference") (OtherBodyIndex :type Integer))
  (bind _door (`self.door`))
  (cast `/Game/ThirdPerson/Blueprints/BP_ThirdPersonCharacter` OtherActor)
  (`self.K2_SetActorLocation` _door (+ (`self.K2_GetActorLocation` _door) (-400.0 0.0 0.0)) false false)
  (`GameplayStatics.PlaySound2D` "/Game/Blueprints/e_folder/AUDIO/impactPlate_medium_000.impactPlate_medium_000" 1.0 1.0 0.0 null null))

(fn `UserConstructionScript`)