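; GI_saveload, a game instance by its name, saves and restores the player's stamina, sprint and shoot flags, and transform through the SG_coding2 save object.
; savegame loads or creates the slot, copies values from BP_ThirdPersonCharacter and writes it back.
; CanShoot overwrites PlayerCanSprint on save, so PlayerCanShoot is never written.
; loadgame applies saved values to the character and teleports it, with debug prints throughout.
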(event `save game`
  (`KismetSystemLibrary.PrintString` "starting save")
  (bind _returnvalue (`GameplayStatics.DoesSaveGameExist` (`self.Slot Name`)))
  (if _returnvalue
    (bind _returnvalue_2 (`GameplayStatics.LoadGameFromSlot` (`self.Slot Name`)))
    (set `self.saving subclass` _returnvalue_2)
    (else
      (bind _returnvalue_3 (`GameplayStatics.CreateSaveGameObject` "/Game/Blueprints/e_folder/SG_coding2.SG_coding2_C"))
      (set `self.saving subclass` _returnvalue_3)))
  (bind _assg_coding_2 (cast `/Game/Blueprints/e_folder/SG_coding2` (`self.saving subclass`)))
  ;[0.2549 0.2356 1] players current data
  (bind _asbp_third_person_character (cast `/Game/ThirdPerson/Blueprints/BP_ThirdPersonCharacter` (`GameplayStatics.GetPlayerCharacter` 0)))
  ;[1 0.9523 0.3138] save game data
  (set `/Game/Blueprints/e_folder/SG_coding2.stamina` (`/Game/ThirdPerson/Blueprints/BP_ThirdPersonCharacter.Stamina` _asbp_third_person_character) _assg_coding_2)
  (bind _output_get (set `/Game/Blueprints/e_folder/SG_coding2.player transform` (`SceneComponent.K2_GetComponentToWorld` (`Character.CapsuleComponent` _asbp_third_person_character)) _assg_coding_2))
  (`KismetSystemLibrary.PrintString` (`KismetStringLibrary.Conv_TransformToString` _output_get))
  (set `/Game/Blueprints/e_folder/SG_coding2.player can sprint` (`/Game/ThirdPerson/Blueprints/BP_ThirdPersonCharacter.CanSprint` _asbp_third_person_character) _assg_coding_2)
  (set `/Game/Blueprints/e_folder/SG_coding2.player can sprint` (`/Game/ThirdPerson/Blueprints/BP_ThirdPersonCharacter.CanShoot` _asbp_third_person_character) _assg_coding_2)
  (`GameplayStatics.SaveGameToSlot` _assg_coding_2 (`self.Slot Name`))
  (`KismetSystemLibrary.PrintString` "succesfully  saved"))

(event `load game`
  (`KismetSystemLibrary.PrintString` "starting load game")
  (bind _returnvalue (`GameplayStatics.DoesSaveGameExist` (`self.Slot Name`)))
  (if _returnvalue
    (bind _returnvalue_2 (`GameplayStatics.LoadGameFromSlot` (`self.Slot Name`)))
    (bind _assg_coding_2 (cast `/Game/Blueprints/e_folder/SG_coding2` _returnvalue_2))
    (bind _asbp_third_person_character (cast `/Game/ThirdPerson/Blueprints/BP_ThirdPersonCharacter` (`GameplayStatics.GetPlayerCharacter` 0)))
    (set `/Game/ThirdPerson/Blueprints/BP_ThirdPersonCharacter.Stamina` (`/Game/Blueprints/e_folder/SG_coding2.stamina` _assg_coding_2) _asbp_third_person_character)
    (set `/Game/ThirdPerson/Blueprints/BP_ThirdPersonCharacter.CanShoot` (`/Game/Blueprints/e_folder/SG_coding2.player can shoot ` _assg_coding_2) _asbp_third_person_character)
    (set `/Game/ThirdPerson/Blueprints/BP_ThirdPersonCharacter.CanSprint` (`/Game/Blueprints/e_folder/SG_coding2.player can sprint` _assg_coding_2) _asbp_third_person_character)
    (bind _player_transform (`/Game/Blueprints/e_folder/SG_coding2.player transform` _assg_coding_2))
    (`KismetSystemLibrary.PrintString` (`KismetStringLibrary.Conv_TransformToString` _player_transform))
    (`Actor.K2_SetActorTransform` _asbp_third_person_character _player_transform false true)
    (`KismetSystemLibrary.PrintString` "success")
    (else
      (`KismetSystemLibrary.PrintString` "Hello"))))