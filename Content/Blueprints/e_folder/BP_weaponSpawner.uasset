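; Weapon spawner actor that creates randomized BP_weapon pickups at its Sphere1 transform.
; It spawns on a repeating two-second Delay loop from BeginPlay and whenever a BP_ThirdPersonCharacter overlaps Sphere1.
; Each spawn copies type, element, base damage, mesh and material from a random DT_weapons row, then calls the weapon's RandomizeValues.
; The spawner's own randomizevalues event is empty, and its text-setting nodes are disconnected.
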(event `self.ReceiveBeginPlay`
  (`KismetSystemLibrary.Delay` 2.0 :!label _label)
  (`self.spawn weapon`)
  (goto _label))

(event `self.Sphere1.OnComponentBeginOverlap`
  (params (OverlappedComponent :type "PrimitiveComponent Object Reference") (OtherActor :type "Actor Object Reference") (OtherComp :type "PrimitiveComponent Object Reference") (OtherBodyIndex :type Integer) (bFromSweep :type Boolean) (SweepResult :type "HitResult Structure (by ref)"))
  (cast `/Game/ThirdPerson/Blueprints/BP_ThirdPersonCharacter` OtherActor)
  (`self.spawn weapon`))

(event `spawn weapon`
  (bind _outrownames (`DataTableFunctionLibrary.GetDataTableRowNames` "/Game/Blueprints/e_folder/dataTables/DT_weapons.DT_weapons"))
  (bind _returnvalue (`|GetDataTableRow` "/Game/Blueprints/e_folder/dataTables/DT_weapons.DT_weapons" (`KismetArrayLibrary.Array_Random` _outrownames))
    (:`then`
      (bind _returnvalue_2 (`|SpawnActorFromClass` "/Game/Blueprints/e_folder/BP_weapon.BP_weapon_C" (`SceneComponent.K2_GetComponentToWorld` (`self.Sphere1`)) "Undefined" "MultiplyWithRoot" null null))
      (set `/Game/Blueprints/e_folder/BP_weapon.weaponType` (break `/Game/Blueprints/e_folder/dataTables/S_weapon` _returnvalue) _returnvalue_2)
      (set `/Game/Blueprints/e_folder/BP_weapon.elementaltype` (`.elementalType_5_2846FDDA4730BDEAAA93CA8DF667B91A` (break `/Game/Blueprints/e_folder/dataTables/S_weapon` _returnvalue)) _returnvalue_2)
      (set `/Game/Blueprints/e_folder/BP_weapon.min damage` (`.basedamage_9_EBDE902B4631FBE2BFB1B5846CCCE4FB` (break `/Game/Blueprints/e_folder/dataTables/S_weapon` _returnvalue)) _returnvalue_2)
      (set `/Game/Blueprints/e_folder/BP_weapon.weopon meshs` (`.weaponmesh_13_DD5BF20D41E95A9DBEA85FA374737501` (break `/Game/Blueprints/e_folder/dataTables/S_weapon` _returnvalue)) _returnvalue_2)
      (`PrimitiveComponent.SetMaterial` (`/Game/Blueprints/e_folder/BP_weapon.weopon body` _returnvalue_2) 0 (`.materialcolor_18_57CE965D4EB73A10071A9B87A9AED05B` (break `/Game/Blueprints/e_folder/dataTables/S_weapon` _returnvalue)))
      (`/Game/Blueprints/e_folder/BP_weapon.randomize values` _returnvalue_2))))

(event `randomize values`)

(fn `UserConstructionScript`)