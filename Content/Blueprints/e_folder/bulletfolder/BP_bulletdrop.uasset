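; Bullet drop test Blueprint that debug-draws a simulated trajectory from its Arrow component alongside the engine's predicted projectile path for comparison.
; Every two seconds it runs a hand-stepped line trace loop, then Predict Projectile Path (Advanced) from the same start and velocity.
; The manual loop adds a fixed downward velocity increment per step, divides only X by SimFrequency, and stops on a hit.
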(event `self.ReceiveBeginPlay`
  (set `self. Start Location` (`SceneComponent.K2_GetComponentLocation` (`self.Arrow`)))
  (`|ExecutionSequence` :!label _label
    (:`then_0`
      (`self.bullet drop calculation`))
    (:`then_1`
      (`GameplayStatics.Blueprint_PredictProjectilePath_Advanced` (make `PredictProjectilePathParams` (`self. Start Location`) (`self.starting velocity`) true 0.0 (`self.Max Sim Time`) true "ECC_WorldStatic" _ _ (`self. Sim Frequency`) 0.0 "ForDuration"))
      (`KismetSystemLibrary.Delay` 2.0)
      (goto _label))))

(event `bullet drop calculation`
  (set `self.Velocity` (`self.starting velocity`))
  (set `self.end` (+ (`self. Start Location`) (/ (`self.Velocity`) (`KismetMathLibrary.MakeVector` (`self. Sim Frequency`) 1.0 1.0))))
  (for _ (range 1 (+ (`KismetMathLibrary.FTrunc` (`self. Sim Frequency`)) 1))
    (bind (_outhit _returnvalue) (`KismetSystemLibrary.LineTraceSingleByProfile` (`self. Start Location`) (`self.end`) "BlockAll"))
    (if _returnvalue
      (`KismetSystemLibrary.PrintString` "hit")
      (break)
      (else
        (`KismetSystemLibrary.DrawDebugLine` (`self. Start Location`) (`self.end`) (struct :`R` 1.0 :`B` 0.275189 :`A` 1.0) (`self.Max Sim Time`) 1.0)
        (`KismetSystemLibrary.DrawDebugSphere` (`self.end`) 5.0 12 (struct :`G` 0.157705 :`B` 1.0 :`A` 1.0) (`self.Max Sim Time`) 1.0)
        (set `self. Start Location` (`self.end`))
        (set `self.Velocity` (+ (`self.Velocity`) (0.0 0.0 -2.4)))
        (set `self.end` (+ (`self. Start Location`) (/ (`self.Velocity`) (`KismetMathLibrary.MakeVector` (`self. Sim Frequency`) 1.0 1.0)))))))
  ;[1 1 1] reset start
  (set `self. Start Location` (`SceneComponent.K2_GetComponentLocation` (`self.Arrow`)))
  (set `self.Velocity` (`self.starting velocity`)))

(fn `UserConstructionScript`)