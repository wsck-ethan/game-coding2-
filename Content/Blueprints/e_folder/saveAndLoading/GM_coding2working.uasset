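; Game mode-style Blueprint (GM_coding2working) that manages per-level save data, using the current level name as the save slot.
; BeginPlay loads or creates an SG_Save object as LevelSave, then calls LoadPlayerLocation and the save object's LoadLevelData.
; Events save LevelSave to its slot or clear its data.
; LoadPlayerLocation is currently empty, with its saved-transform and PlayerStart fallback logic left disconnected.
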(event `SaveLevelData`
  ;[0.1615 0.1615 0.1615] Save Level Data
  (bind _returnvalue (`GameplayStatics.GetCurrentLevelName` true))
  (`GameplayStatics.SaveGameToSlot` (`self.levelSave`) _returnvalue)
  (`KismetSystemLibrary.PrintString` "Saved game to slot"))

(event `self.ReceiveBeginPlay`
  ;[0.05313 0.05313 0.05313] Beginning Of Level
  (`|ExecutionSequence`
    (:`then_1`
      (bind _returnvalue (`GameplayStatics.GetCurrentLevelName` true))
      ;;[0.1531 0.1531 0.1531] Initialize Level Data
      (bind _returnvalue_2 (`GameplayStatics.DoesSaveGameExist` _returnvalue))
      (if _returnvalue_2
        (bind _returnvalue_3 (`GameplayStatics.LoadGameFromSlot` _returnvalue))
        (bind _assg_save (cast `/Game/Blueprints/e_folder/saveAndLoading/SG_Save` _returnvalue_3))
        (set `self.levelSave` _assg_save)
        (else
          (bind _returnvalue_4 (`GameplayStatics.CreateSaveGameObject` "/Game/Blueprints/e_folder/saveAndLoading/SG_Save.SG_Save_C"))
          (set `self.levelSave` _returnvalue_4)))
      (`self.load player location`)
      (`/Game/Blueprints/e_folder/saveAndLoading/SG_Save.load level data` (`self.levelSave`)))))

(event `DeleteLevelData`
  ;[0.3115 0.3115 0.3115] Delete Level Data
  (bind _levelsave (`self.levelSave`)
    (:`then`
      (`/Game/Blueprints/e_folder/saveAndLoading/SG_Save.cleardata` _levelsave))
    (:`else`)))

(fn `load player location`)

(fn `UserConstructionScript`)